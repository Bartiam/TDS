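; Freight elevator actor that rises once, the first time a BP_TDSCharacter overlaps it.
; The overlap sets IsElevatorUp and starts a fast looping timer on UpElevator.
; Each tick of that timer writes CurrentLocationZ to the root's world Z and increments it, clearing the timer at MaxLocationZ.
; The file has no descent or reset, and CurrentLocationZ is not read from the actor's placed height.
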(event `self.ReceiveActorBeginOverlap`
  (params (OtherActor :type "Actor Object Reference"))
  (cast `/Game/Blueprints/Character/BP_TDSCharacter` OtherActor)
  (if (not (`self.bIsElevatorUp`))
    (set `self.bIsElevatorUp` true)
    (`KismetSystemLibrary.K2_SetTimer` null "UpElevator" 0.01 true)))

(fn `UpElevator`
  (bind _defaultsceneroot (`self.DefaultSceneRoot`))
  (bind (_returnvalue_x _returnvalue_y) (`KismetMathLibrary.BreakVector` (`SceneComponent.K2_GetComponentLocation` _defaultsceneroot)))
  (`SceneComponent.K2_SetWorldLocation` _defaultsceneroot (`KismetMathLibrary.MakeVector` _returnvalue_x _returnvalue_y (`self.CurrentLocationZ`)) false false)
  (`/Engine/EditorBlueprintResources/StandardMacros.IncrementFloat` (`self.CurrentLocationZ`)
    (:`  `
      (if (>= (`self.CurrentLocationZ`) (`self.MaxLocationZ`))
        (`KismetSystemLibrary.K2_ClearTimer` null "UpElevator")))))

(fn `UserConstructionScript`)