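; Vertical sliding door that lowers to open when a BP_TDSCharacter overlaps its enter trigger and rises to close when one overlaps its exit trigger.
; An IsDoorOpen flag gates both triggers, each starting a looping timer by function name.
; OpenDoor and CloseDoor step the door's world Z by one unit per timer call until it reaches its limit, then clear the timer and update the flag.
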(event `self.EnterTrigger.OnComponentBeginOverlap`
  (params (OverlappedComponent :type "PrimitiveComponent Object Reference") (OtherActor :type "Actor Object Reference") (OtherComp :type "PrimitiveComponent Object Reference") (OtherBodyIndex :type Integer) (bFromSweep :type Boolean) (SweepResult :type "HitResult Structure (by ref)"))
  (cast `/Game/Blueprints/Character/BP_TDSCharacter` OtherActor)
  (if (not (`self.bIsDoorOpen`))
    (`KismetSystemLibrary.K2_SetTimer` null "OpenDoor" 0.005 true)))

(event `self.ExitTrigger.OnComponentBeginOverlap`
  (params (OverlappedComponent :type "PrimitiveComponent Object Reference") (OtherActor :type "Actor Object Reference") (OtherComp :type "PrimitiveComponent Object Reference") (OtherBodyIndex :type Integer) (bFromSweep :type Boolean) (SweepResult :type "HitResult Structure (by ref)"))
  (cast `/Game/Blueprints/Character/BP_TDSCharacter` OtherActor)
  (if (`self.bIsDoorOpen`)
    (`KismetSystemLibrary.K2_SetTimer` null "CloseDoor" 0.005 true)))

(fn `CloseDoor`
  (bind _door (`self.Door`))
  (bind _currentlocationdoorz (`self.CurrentLocationDoorZ`))
  (bind (_returnvalue_x _returnvalue_y) (`KismetMathLibrary.BreakVector` (`SceneComponent.K2_GetComponentLocation` _door)))
  (`SceneComponent.K2_SetWorldLocation` _door (`KismetMathLibrary.MakeVector` _returnvalue_x _returnvalue_y _currentlocationdoorz) false false)
  (`/Engine/EditorBlueprintResources/StandardMacros.IncrementFloat` _currentlocationdoorz
    (:`  `
      (if (>= _currentlocationdoorz (`self.MaxLocationDoorZ`))
        (`KismetSystemLibrary.K2_ClearTimer` null "CloseDoor")
        (set `self.bIsDoorOpen` false)))))

(fn `OpenDoor`
  (bind _door (`self.Door`))
  (bind _currentlocationdoorz (`self.CurrentLocationDoorZ`))
  (bind (_returnvalue_x _returnvalue_y) (`KismetMathLibrary.BreakVector` (`SceneComponent.K2_GetComponentLocation` _door)))
  (`SceneComponent.K2_SetWorldLocation` _door (`KismetMathLibrary.MakeVector` _returnvalue_x _returnvalue_y _currentlocationdoorz) false false)
  (`/Engine/EditorBlueprintResources/StandardMacros.DecrementFloat` _currentlocationdoorz
    (:`  `
      (if (<= _currentlocationdoorz (`self.MinLocationDoorZ`))
        (`KismetSystemLibrary.K2_ClearTimer` null "OpenDoor")
        (set `self.bIsDoorOpen` true)))))

(fn `UserConstructionScript`)