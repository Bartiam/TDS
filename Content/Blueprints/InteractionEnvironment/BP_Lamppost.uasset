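; BP_Lamppost is an environment lamppost whose spotlight is configured when play begins.
; If the lamp is on, it makes the SpotLight visible and, for flashing lampposts, assigns the M_Flashing light function material so the flicker comes from the material rather than Blueprint logic.
; If it is off, it destroys the SpotLight and LampWorkCue components.
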(event `self.ReceiveBeginPlay`
  (if (`self.bIsLamppostOn`)
    (`SceneComponent.SetVisibility` (`self.SpotLight`) true false)
    (if (`self.bIsFlashingLampost`)
      (`LightComponent.SetLightFunctionMaterial` (`self.SpotLight`) "/Game/SoulCity/Environment/Materials/LamppostMat/M_Flashing.M_Flashing"))
    (else
      (`ActorComponent.K2_DestroyComponent` (`self.LampWork_Cue`))
      (`ActorComponent.K2_DestroyComponent` (`self.SpotLight`)))))

(fn `UserConstructionScript`)