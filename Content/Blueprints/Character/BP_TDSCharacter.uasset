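; Top-down player character Blueprint with movement states, a configurable camera boom and hotkey-triggered animations.
; Walking, Running and Aiming inputs toggle state flags, then call ChangeMovementState.
; The construction script applies height, rotation and lag settings to the boom.
; Hard-wired keys play hip or ironsight fire montages, a death montage and a world camera shake, while Tick prints current stamina for debugging.
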(event `Key|SpaceBar`
  (params (Key :type "Key Structure"))
  (bind _mesh (`self.Mesh`))
  (:`Pressed`
    (if (`self.bIsAiming`)
      (`|PlayMontage` _mesh "/Game/Blueprints/Character/Mannequin/Animations/CharacterAnim/AnimFire_Rifle_Ironsights_Montage.AnimFire_Rifle_Ironsights_Montage")
      (else
        (`|PlayMontage` _mesh "/Game/Blueprints/Character/Mannequin/Animations/CharacterAnim/AnimFire_Rifle_Hip_Montage.AnimFire_Rifle_Hip_Montage")))))

(event `Key|V`
  (params (Key :type "Key Structure"))
  (:`Pressed`
    (`|PlayMontage` (`self.Mesh`) "/Game/Blueprints/Character/Mannequin/Animations/CharacterAnim/AnimDeath_1_Montage.AnimDeath_1_Montage")))

(event `Key|F`
  (params (Key :type "Key Structure"))
  (:`Pressed`
    (`self.CameraShakeEvent`)))

(event `self.ReceiveTick`
  (params (DeltaSeconds :type "Float (single-precision)"))
  (`KismetSystemLibrary.PrintString` (`KismetStringLibrary.Conv_DoubleToString` (`self.GetCurrentStamina`))))

(event `InputAction|Walking`
  (params (Key :type "Key Structure"))
  (:`Pressed`
    (set `self.bIsWalking` true)
    (`self.ChangeMovementState` :!label _label))
  (:`Released`
    (set `self.bIsWalking` false)
    (goto _label)))

(event `InputAction|Running`
  (params (Key :type "Key Structure"))
  (:`Pressed`
    (set `self.bIsFastRunning` true)
    (`self.ChangeMovementState` :!label _label_2))
  (:`Released`
    (set `self.bIsFastRunning` false)
    (goto _label_2)))

(event `InputAction|Aiming`
  (params (Key :type "Key Structure"))
  (:`Pressed`
    (set `self.bIsAiming` true)
    (`self.ChangeMovementState` :!label _label_3))
  (:`Released`
    (set `self.bIsAiming` false)
    (goto _label_3)))

(fn `CameraShakeEvent`
  (`GameplayStatics.PlayWorldCameraShake` "/Game/Blueprints/Game/BP_ShakeCamera.BP_ShakeCamera_C" (`SceneComponent.K2_GetComponentLocation` (`self.TopDownCameraComponent`)) 0.0 30.0))

(fn `UserConstructionScript`
  (bind _cameraboom (`self.CameraBoom`))
  (set `SpringArmComponent.TargetArmLength` (`self.minCameraHeight`) _cameraboom)
  (`SceneComponent.K2_SetRelativeRotation` _cameraboom (`self.rotateOfCamera`) false false)
  (set `SpringArmComponent.bEnableCameraLag` (`self.flow`) _cameraboom)
  (set `SpringArmComponent.CameraLagSpeed` (`self.coefSmooth`) _cameraboom))